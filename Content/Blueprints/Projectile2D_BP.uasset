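; Projectile Blueprint that aims itself on BeginPlay at a predicted 2D trajectory against a target with hard-coded start position, heading and speed.
; It passes its speed, pitch and XZ start position to PredictTrajectory2D.
; On success it applies the resulting pitch, records the start time and sizes its collision sphere from velocity and rotation speed.
; Debug prints show the angle and wait time, or report an impossible solution.
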(event EventBeginPlay
  (bind _startlocation (Variables|Default|GetStartLocation))
  (bind (_resultangle _returnvalue) (Class|Projectile2D|PredictTrajectory2D (Variables|Default|GetVelocity) 2e+02 (.pitch (Variables|Default|GetStartRotation)) 7e+01 (Utilities|Array|MakeArray (.x _startlocation) (.z _startlocation)) (Utilities|Array|MakeArray -1.74e+03 5.34e+03) 0.1))
  (if _returnvalue
    (Variables|Default|SetStartRotation (Math|Rotator|MakeRotator 0.0 _resultangle 0.0))
    (Transformation|SetActorRotation (Math|Rotator|MakeRotator 0.0 _resultangle 0.0))
    (Development|PrintString (Utilities|String|ToString(Float) _resultangle) true true "(R=0.000000,G=0.660000,B=1.000000,A=1.000000)" 1e+01)
    (Development|PrintString (Utilities|String|ToString(Float) (Variables|Default|GetWaitTime)) true true "(R=0.074769,G=1.000000,B=0.000000,A=1.000000)" 1e+01)
    (Variables|Default|SetTrajectoryStartMoment (Utilities|Time|GetTimeSeconds))
    (Components|Sphere|SetSphereRadius (Variables|Default|GetSphere) (+ (* (/ 9e+01 (Variables|Default|GetRotationSpeed)) (Variables|Default|GetVelocity)) 5.0) true)
    (else
      (Development|PrintString "Impossible" true true "(R=0.000000,G=0.660000,B=1.000000,A=1.000000)" 1e+01))))

(fn ConstructionScript)