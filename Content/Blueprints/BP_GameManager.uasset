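; BP_GameManager sets up 2D and 3D projectile-versus-target simulations, spawning both actors with shared gravity and simulation speed.
; ParabolaParabola solvers gate the 2D and 3D runs, printing "Impossible" on failure; 3D passes predicted rotation and wait time on.
; SetupLauncher places a ballistic or missile launcher on traced ground and links the projectile.
; Separate Init functions spawn full launcher-projectile-target sets, though ProjectileInit3D still uses 2D classes and solver.
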(fn ConstructionScript)

(fn 2D
  (bind _t (Variables|Default|GetT))
  (bind _p (Variables|Default|GetP))
  (bind _returnvalue (Game|SpawnActorfromClass "/Game/Blueprints/BP_Target2D.BP_Target2D_C" (Math|Transform|MakeTransform "0, 0, 0" "0, 0, 0" "1,1,1") "Undefined" 0 0))
  (Class|Target2D|InitializeTarget2D _returnvalue _t (Variables|Default|GetG) (Variables|Default|GetWorldSimulationSpeed))
  (bind _returnvalue_2 (Game|SpawnActorfromClass "/Game/Blueprints/BP_Projectile2D.BP_Projectile2D_C" (Math|Transform|MakeTransform "0, 0, 0" "0, 0, 0" "1,1,1") "Undefined" 0 0))
  (bind _returnvalue_3 (Class|GameManager|ParabolaParabola2D _p _t 0.1))
  (if _returnvalue_3
    (Class|Projectile2D|InitializeProjectile2D _returnvalue_2 _p _returnvalue (Variables|Default|GetG) (Variables|Default|GetWorldSimulationSpeed))
    (Development|PrintString (Utilities|String|ToString(Rotator) (Variables|/Script/TUI2023.Projectile2D|GetDesiredRotation _returnvalue_2)) true true "(R=0.000000,G=0.660000,B=1.000000,A=1.000000)" 15.0)
    (else
      (Development|PrintString "Impossible" true true "(R=0.000000,G=0.660000,B=1.000000,A=1.000000)" 5.0))))

(fn 3D
  (bind _p3d (Variables|Default|GetP3D))
  (bind _returnvalue (Class|GameManager|ParabolaParabola3D (Variables|Default|GetP3D) (Variables|Default|GetT3D) 0.1))
  (if _returnvalue
    (bind _returnvalue_2 (Game|SpawnActorfromClass "/Game/Blueprints/BP_Target3D.BP_Target3D_C" (Math|Transform|MakeTransform "0, 0, 0" "0, 0, 0" "1,1,1") "Undefined" 0 0))
    (Class|Target3D|InitializeTarget3D _returnvalue_2 (Variables|Default|GetT3D) (Variables|Default|GetG) (Variables|Default|GetWorldSimulationSpeed))
    (bind _returnvalue_3 (Game|SpawnActorfromClass "/Game/Blueprints/BP_Projectile3D.BP_Projectile3D_C" (Math|Transform|MakeTransform "0, 0, 0" "0, 0, 0" "1,1,1") "Undefined" 0 0))
    (Class|Projectile3D|SetPredictionResults _returnvalue_3 (.desiredrotation _p3d) (.waittime _p3d))
    (Class|Projectile3D|InitializeProjectile3D _returnvalue_3 (Variables|Default|GetP3D) _returnvalue_2 (Variables|Default|GetG) (Variables|Default|GetWorldSimulationSpeed))
    (Development|PrintString (Utilities|String|ToString(Float) (.waittime _p3d)) true true "(R=0.200661,G=0.760417,B=0.000000,A=1.000000)" 3e+01)
    (CallFunction|SetupLauncher (Variables|Default|GetP3D) _returnvalue_3)
    (else
      (Development|PrintString "Impossible" true true "(R=0.000000,G=0.660000,B=1.000000,A=1.000000)" 5.0))))

(fn SetupLauncher
  (params (ProjectileParameters :type Projectile%20Params%20Structure%20%28by%20ref%29) (ProjectileRef :type Actor%20Object%20Reference%20%28by%20ref%29))
  (bind (_x _y) (Math|Vector|BreakVector "0, 0, 0"))
  (LocalVariables|SetProjectile ProjectileRef)
  (bind _output_get (LocalVariables|SetParams ProjectileParameters))
  (if (.isballistic _output_get)
    (bind _outhit (Collision|LineTraceByChannel (Math|Vector|MakeVector _x _y 1e+04) (Math|Vector|MakeVector _x _y -1.5e+03) "TraceTypeQuery1" false (Utilities|Array|MakeArray (LocalVariables|GetProjectile)) "None"))
    (bind _returnvalue (Game|SpawnActorfromClass "/Game/Blueprints/BP_ProjectileLauncher.BP_ProjectileLauncher_C" (Math|Transform|MakeTransform (Math|Vector|MakeVector (.X (Math|Vector|BreakVector (.Location (Collision|BreakHitResult _outhit)))) (.Y (Math|Vector|BreakVector (.Location (Collision|BreakHitResult _outhit)))) (+ (.Z (Math|Vector|BreakVector (.Location (Collision|BreakHitResult _outhit)))) (* 1.0 (.sizek (LocalVariables|GetParams))))) "0, 0, 0" "1,1,1") "AlwaysSpawn" 0 0))
    (Default|SetActorRotationAdvanced _returnvalue (.startrotation (LocalVariables|GetParams)))
    (Variables|/Game/Blueprints/BP_ProjectileLauncher.BP_ProjectileLauncher_C|SetDesiredRotation _returnvalue (.desiredrotation (LocalVariables|GetParams)))
    (Variables|/Game/Blueprints/BP_ProjectileLauncher.BP_ProjectileLauncher_C|SetWaitTime _returnvalue (.waittime (LocalVariables|GetParams)))
    (bind _output_get_2 (Variables|/Game/Blueprints/BP_ProjectileLauncher.BP_ProjectileLauncher_C|SetSizeK _returnvalue (.sizek (LocalVariables|GetParams))))
    (Variables|/Game/Blueprints/BP_ProjectileLauncher.BP_ProjectileLauncher_C|SetProjectileRef _returnvalue (LocalVariables|GetProjectile))
    (Transformation|SetWorldScale3D (Variables|/Script/Engine.Actor|GetRootComponent _returnvalue) (Math|Vector|MakeVector _output_get_2 _output_get_2 _output_get_2))
    (else
      (bind _outhit_2 (Collision|LineTraceByChannel (Math|Vector|MakeVector (.X (Math|Vector|BreakVector (.startlocation _output_get))) (.Y (Math|Vector|BreakVector (.startlocation _output_get))) 1e+04) (Math|Vector|MakeVector (.X (Math|Vector|BreakVector (.startlocation _output_get))) (.Y (Math|Vector|BreakVector (.startlocation _output_get))) -1.5e+03) "TraceTypeQuery1" false (Utilities|Array|MakeArray (LocalVariables|GetProjectile)) "None"))
      (bind _returnvalue_2 (Game|SpawnActorfromClass "/Game/Blueprints/BP_MissileLauncher.BP_MissileLauncher_C" (Math|Transform|MakeTransform (Math|Vector|MakeVector (.X (Math|Vector|BreakVector (.Location (Collision|BreakHitResult _outhit_2)))) (.Y (Math|Vector|BreakVector (.Location (Collision|BreakHitResult _outhit_2)))) (+ (.Z (Math|Vector|BreakVector (.Location (Collision|BreakHitResult _outhit_2)))) (* 1.0 (.sizek (LocalVariables|GetParams))))) "0, 0, 0" "1,1,1") "AlwaysSpawn" 0 0))
      (Default|SetActorRotationAdvanced _returnvalue_2 (.startrotation (LocalVariables|GetParams)))
      (Variables|/Game/Blueprints/BP_MissileLauncher.BP_MissileLauncher_C|SetDesiredRotation _returnvalue_2 (.desiredrotation (LocalVariables|GetParams)))
      (Variables|/Game/Blueprints/BP_MissileLauncher.BP_MissileLauncher_C|SetWaitTime _returnvalue_2 0.0)
      (bind _output_get_3 (Variables|/Game/Blueprints/BP_MissileLauncher.BP_MissileLauncher_C|SetSizeK _returnvalue_2 0.0))
      (Variables|/Game/Blueprints/BP_MissileLauncher.BP_MissileLauncher_C|SetMissileRef _returnvalue_2 (LocalVariables|GetProjectile))
      (Transformation|SetWorldScale3D (Variables|/Script/Engine.Actor|GetRootComponent _returnvalue_2) (Math|Vector|MakeVector _output_get_3 _output_get_3 _output_get_3)))))

(fn ProjectileInit2D
  (params (ProjectileParams :type Projectile%20Params%20Structure) (TargetParams :type Target%20Params%20Structure))
  (LocalVariables|SetProjectile ProjectileParams)
  (LocalVariables|SetTarget TargetParams)
  (bind _outhit (Collision|LineTraceByChannel (Math|Vector|MakeVector (.X (Math|Vector|BreakVector (.startlocation (LocalVariables|GetProjectile)))) 0.0 1e+04) (Math|Vector|MakeVector (.X (Math|Vector|BreakVector (.startlocation (LocalVariables|GetProjectile)))) 0.0 -1.5e+03) "TraceTypeQuery1" false 0 "None"))
  (bind _returnvalue (Game|SpawnActorfromClass "/Game/Blueprints/BP_ProjectileLauncher.BP_ProjectileLauncher_C" (Math|Transform|MakeTransform (Math|Vector|MakeVector (.X (Math|Vector|BreakVector (.Location (Collision|BreakHitResult _outhit)))) 0.0 (+ (.Z (Math|Vector|BreakVector (.Location (Collision|BreakHitResult _outhit)))) (* 1.0 (.sizek (LocalVariables|GetProjectile))))) "0, 0, 0" (Math|Conversions|ToVector(Float) (.sizek (LocalVariables|GetProjectile)))) "AlwaysSpawn" 0 0))
  (Default|SetActorRotationAdvanced _returnvalue (.startrotation (LocalVariables|GetProjectile)))
  (Variables|/Game/Blueprints/BP_ProjectileLauncher.BP_ProjectileLauncher_C|SetDesiredRotation _returnvalue (.desiredrotation (LocalVariables|GetProjectile)))
  (Variables|/Game/Blueprints/BP_ProjectileLauncher.BP_ProjectileLauncher_C|SetWaitTime _returnvalue (.waittime (LocalVariables|GetProjectile)))
  (bind _output_get (Variables|/Game/Blueprints/BP_ProjectileLauncher.BP_ProjectileLauncher_C|SetSizeK _returnvalue (.sizek (LocalVariables|GetProjectile))))
  (Transformation|SetWorldScale3D (Variables|/Script/Engine.Actor|GetRootComponent _returnvalue) (Math|Conversions|ToVector(Float) _output_get))
  (Class|GameManager|ParabolaParabola2D (LocalVariables|GetProjectile) (LocalVariables|GetTarget) 0.1)
  (bind _returnvalue_2 (Game|SpawnActorfromClass "/Game/Blueprints/BP_Projectile2D.BP_Projectile2D_C" (Math|Transform|MakeTransform (Math|Vector|MakeVector (.x (.startlocation (LocalVariables|GetProjectile))) 0.0 (.z (.startlocation (LocalVariables|GetProjectile)))) (.startrotation (LocalVariables|GetProjectile)) (Math|Conversions|ToVector(Float) (.sizek (LocalVariables|GetProjectile)))) "Undefined" 0 0))
  (bind _returnvalue_3 (Game|SpawnActorfromClass "/Game/Blueprints/BP_Target2D.BP_Target2D_C" (Math|Transform|MakeTransform (Math|Vector|MakeVector (.x (.startlocation (LocalVariables|GetTarget))) 0.0 (.z (.startlocation (LocalVariables|GetTarget)))) (.startrotation (LocalVariables|GetTarget)) (Math|Conversions|ToVector(Float) (.sizek (LocalVariables|GetTarget)))) "Undefined" 0 0))
  (Variables|/Game/Blueprints/BP_ProjectileLauncher.BP_ProjectileLauncher_C|SetProjectileRef _returnvalue _returnvalue_2)
  (Class|Projectile2D|InitializeProjectile2D _returnvalue_2 (LocalVariables|GetProjectile) _returnvalue_3 (Variables|Default|GetG) (Variables|Default|GetWorldSimulationSpeed))
  (Class|Target2D|InitializeTarget2D _returnvalue_3 (LocalVariables|GetTarget) (Variables|Default|GetG) (Variables|Default|GetWorldSimulationSpeed)))

(fn ProjectileInit3D
  (params (ProjectileParams :type Projectile%20Params%20Structure) (TargetParams :type Target%20Params%20Structure))
  (LocalVariables|SetProjectile ProjectileParams)
  (LocalVariables|SetTarget TargetParams)
  (bind _outhit (Collision|LineTraceByChannel (Math|Vector|MakeVector (.X (Math|Vector|BreakVector (.startlocation (LocalVariables|GetProjectile)))) (.Y (Math|Vector|BreakVector (.startlocation (LocalVariables|GetProjectile)))) 1e+04) (Math|Vector|MakeVector (.X (Math|Vector|BreakVector (.startlocation (LocalVariables|GetProjectile)))) (.Y (Math|Vector|BreakVector (.startlocation (LocalVariables|GetProjectile)))) -1.5e+03) "TraceTypeQuery1" false 0 "None"))
  (bind _returnvalue (Game|SpawnActorfromClass "/Game/Blueprints/BP_ProjectileLauncher.BP_ProjectileLauncher_C" (Math|Transform|MakeTransform (Math|Vector|MakeVector (.X (Math|Vector|BreakVector (.Location (Collision|BreakHitResult _outhit)))) (.Y (Math|Vector|BreakVector (.Location (Collision|BreakHitResult _outhit)))) (+ (.Z (Math|Vector|BreakVector (.Location (Collision|BreakHitResult _outhit)))) (* 1.0 (.sizek (LocalVariables|GetProjectile))))) "0, 0, 0" (Math|Conversions|ToVector(Float) (.sizek (LocalVariables|GetProjectile)))) "AlwaysSpawn" 0 0))
  (Default|SetActorRotationAdvanced _returnvalue (.startrotation (LocalVariables|GetProjectile)))
  (Variables|/Game/Blueprints/BP_ProjectileLauncher.BP_ProjectileLauncher_C|SetDesiredRotation _returnvalue (.desiredrotation (LocalVariables|GetProjectile)))
  (Variables|/Game/Blueprints/BP_ProjectileLauncher.BP_ProjectileLauncher_C|SetWaitTime _returnvalue (.waittime (LocalVariables|GetProjectile)))
  (bind _output_get (Variables|/Game/Blueprints/BP_ProjectileLauncher.BP_ProjectileLauncher_C|SetSizeK _returnvalue (.sizek (LocalVariables|GetProjectile))))
  (Transformation|SetWorldScale3D (Variables|/Script/Engine.Actor|GetRootComponent _returnvalue) (Math|Conversions|ToVector(Float) _output_get))
  (Class|GameManager|ParabolaParabola2D (LocalVariables|GetProjectile) (LocalVariables|GetTarget) 0.1)
  (bind _returnvalue_2 (Game|SpawnActorfromClass "/Game/Blueprints/BP_Projectile2D.BP_Projectile2D_C" (Math|Transform|MakeTransform (.startlocation (LocalVariables|GetProjectile)) (.startrotation (LocalVariables|GetProjectile)) (Math|Conversions|ToVector(Float) (.sizek (LocalVariables|GetProjectile)))) "Undefined" 0 0))
  (bind _returnvalue_3 (Game|SpawnActorfromClass "/Game/Blueprints/BP_Target2D.BP_Target2D_C" (Math|Transform|MakeTransform (.startlocation (LocalVariables|GetTarget)) (.startrotation (LocalVariables|GetTarget)) (Math|Conversions|ToVector(Float) (.sizek (LocalVariables|GetTarget)))) "Undefined" 0 0))
  (Variables|/Game/Blueprints/BP_ProjectileLauncher.BP_ProjectileLauncher_C|SetProjectileRef _returnvalue _returnvalue_2)
  (Class|Projectile2D|InitializeProjectile2D _returnvalue_2 (LocalVariables|GetProjectile) _returnvalue_3 (Variables|Default|GetG) (Variables|Default|GetWorldSimulationSpeed))
  (Class|Target2D|InitializeTarget2D _returnvalue_3 (LocalVariables|GetTarget) (Variables|Default|GetG) (Variables|Default|GetWorldSimulationSpeed)))

(fn MissileInit2D
  (params (MissileParams :type Projectile%20Params%20Structure) (TargetParams :type Target%20Params%20Structure))
  (LocalVariables|SetMissile MissileParams)
  (LocalVariables|SetTarget TargetParams)
  (bind _outhit (Collision|LineTraceByChannel (Math|Vector|MakeVector (.X (Math|Vector|BreakVector (.startlocation (LocalVariables|GetMissile)))) 0.0 1e+04) (Math|Vector|MakeVector (.X (Math|Vector|BreakVector (.startlocation (LocalVariables|GetMissile)))) 0.0 -1.5e+03) "TraceTypeQuery1" false 0 "None"))
  (bind _returnvalue (Game|SpawnActorfromClass "/Game/Blueprints/BP_MissileLauncher.BP_MissileLauncher_C" (Math|Transform|MakeTransform (Math|Vector|MakeVector (.X (Math|Vector|BreakVector (.Location (Collision|BreakHitResult _outhit)))) 0.0 (+ (.Z (Math|Vector|BreakVector (.Location (Collision|BreakHitResult _outhit)))) (* 1.0 (.sizek (LocalVariables|GetMissile))))) "0, 0, 0" (Math|Conversions|ToVector(Float) (.sizek (LocalVariables|GetMissile)))) "AlwaysSpawn" 0 0))
  (Default|SetActorRotationAdvanced _returnvalue (.startrotation (LocalVariables|GetMissile)))
  (Variables|/Game/Blueprints/BP_MissileLauncher.BP_MissileLauncher_C|SetDesiredRotation _returnvalue (.desiredrotation (LocalVariables|GetMissile)))
  (Variables|/Game/Blueprints/BP_MissileLauncher.BP_MissileLauncher_C|SetWaitTime _returnvalue (.waittime (LocalVariables|GetMissile)))
  (Variables|/Game/Blueprints/BP_MissileLauncher.BP_MissileLauncher_C|SetSizeK _returnvalue (.sizek (LocalVariables|GetMissile)))
  (Transformation|SetWorldScale3D (Variables|/Script/Engine.Actor|GetRootComponent _returnvalue) (Math|Conversions|ToVector(Float) (.sizek (LocalVariables|GetMissile))))
  (bind _returnvalue_2 (Game|SpawnActorfromClass "/Game/Blueprints/BP_Projectile2D.BP_Projectile2D_C" (Math|Transform|MakeTransform (Math|Vector|MakeVector (.x (.startlocation (LocalVariables|GetMissile))) 0.0 (.z (.startlocation (LocalVariables|GetMissile)))) (.startrotation (LocalVariables|GetMissile)) (Math|Conversions|ToVector(Float) (.sizek (LocalVariables|GetMissile)))) "Undefined" 0 0))
  (bind _returnvalue_3 (Game|SpawnActorfromClass "/Game/Blueprints/BP_Target2D.BP_Target2D_C" (Math|Transform|MakeTransform (Math|Vector|MakeVector (.x (.startlocation (LocalVariables|GetTarget))) 0.0 (.z (.startlocation (LocalVariables|GetTarget)))) (.startrotation (LocalVariables|GetTarget)) (Math|Conversions|ToVector(Float) (.sizek (LocalVariables|GetTarget)))) "Undefined" 0 0))
  (Variables|/Game/Blueprints/BP_MissileLauncher.BP_MissileLauncher_C|SetMissileRef _returnvalue _returnvalue_2)
  (Class|Projectile2D|InitializeProjectile2D _returnvalue_2 (LocalVariables|GetMissile) _returnvalue_3 (Variables|Default|GetG) (Variables|Default|GetWorldSimulationSpeed))
  (Class|Target2D|InitializeTarget2D _returnvalue_3 (LocalVariables|GetTarget) (Variables|Default|GetG) (Variables|Default|GetWorldSimulationSpeed)))