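; Missile launcher actor that aims its turret along a referenced projectile's rotation during an initial wait period.
; Until WaitTime elapses, Tick checks the gun against DesiredRotation; while they differ, it copies the projectile's rotation and pins the projectile to the gun's location.
; SetActorRotationAdvanced splits rotation into yaw for RotatingBase and pitch plus yaw for Gun.
; Tick disables itself afterward; a debug line trace is left disconnected.
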(event EventTick
  (params (DeltaSeconds :type Float%20%28single-precision%29))
  (if (>= (Actor|GetGameTimeSinceCreation) (Variables|Default|GetWaitTime))
    (Actor|Tick|SetActorTickEnabled false)
    (elif (Utilities|Enum|NotEqual(Enum) (Transformation|GetWorldRotation (Variables|Default|GetGun)) (Variables|Default|GetDesiredRotation) 0.0)
      (CallFunction|SetActorRotationAdvanced (Transformation|GetActorRotation (Variables|Default|GetProjectileRef)))
      (Transformation|SetActorLocation (Variables|Default|GetProjectileRef) (Transformation|GetWorldLocation (Variables|Default|GetGun)) false false))))

(fn ConstructionScript)

(fn SetActorRotationAdvanced
  (params (NewRotation :type Rotator))
  (Transformation|SetWorldRotation (Variables|Default|GetRotatingBase) (Math|Rotator|MakeRotator 0.0 0.0 (.yaw NewRotation)) false false)
  (Transformation|SetWorldRotation (Variables|Default|GetGun) (Math|Rotator|MakeRotator 0.0 (.pitch NewRotation) (.yaw NewRotation)) false false))